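; BP_Onyx_SwordMaster is a player character Blueprint that sets up its camera through the Gameplay Cameras system.
; On BeginPlay it caches the player controller, activates the camera component, then adds persistent global and base rigs for defaults and collision offset.
; It supplies camera properties from its style and crouch stance, while camera mode selection uses constant conditions, so it always yields one mode.
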(event `self.ReceiveBeginPlay`
  (`parent.ReceiveBeginPlay`)
  (bind _asplayer_controller (cast `PlayerController` (`self.GetController`)))
  (set `self.Player Controller` _asplayer_controller)
  (`GameplayCameraComponent.ActivateCameraForPlayerController` (`self.GameplayCamera`) (`self.Player Controller`))
  (`ActivateCameraRigFunctions.ActivatePersistentGlobalCameraRig` (`self.Player Controller`) "/Game/Blueprints/Cameras/CameraRig_BaseDefaults.CameraRig_BaseDefaults")
  (`ActivateCameraRigFunctions.ActivatePersistentBaseCameraRig` (`self.Player Controller`) "/Game/Blueprints/Cameras/CameraRig_CollisionOffset.CameraRig_CollisionOffset"))

(event `self.ReceiveTick`
  (params (DeltaSeconds :type "Float (single-precision)"))
  (`parent.ReceiveTick` DeltaSeconds))

(fn `Get_CharacterPropertiesForCamera`
  (returns (ReturnValue :type "/Game/Blueprints/Cameras/S_CharacterPropertiesForCamera Structure"))
  (return (make `/Game/Blueprints/Cameras/S_CharacterPropertiesForCamera` (`self.CameraStyle`) (select `bool` true :`false` (select `bool` true :`false` "NewEnumerator0" :`true` "NewEnumerator1" :!type "/Game/Blueprints/Cameras/E_CameraMode Enum") :`true` "NewEnumerator2") (select `bool` (`NavMovementInterface.IsCrouching` (`self.CharacterMovement`)) :`false` "NewEnumerator0" :`true` "NewEnumerator1" :!type "/Game/Blueprints/Data/E_Stance Enum"))))

(fn `UserConstructionScript`
  (`parent.UserConstructionScript`))